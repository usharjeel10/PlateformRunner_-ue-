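; BP_PointsSpawn is a short-lived platformer actor that shows a floating points value.
; On BeginPlay it gets the points widget from its widget component, plays its points animation and sets the text to PointsToAdd.
; It waits for the animation's length, then destroys itself.
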(event `self.ReceiveBeginPlay`
  (bind _aspoints (cast `/Game/Platformer/UI/points` (`WidgetComponent.GetWidget` (`self.Widget`))))
  (bind _pointsanim (`/Game/Platformer/UI/points.pointsAnim` _aspoints))
  (`UserWidget.PlayAnimation` _aspoints _pointsanim 0.0 1 "Forward" 1.0 false)
  (`TextBlock.SetText` (`/Game/Platformer/UI/points.pointsText` _aspoints) (`KismetTextLibrary.Conv_IntToText` (`self.pointsToAdd`)))
  (`KismetSystemLibrary.Delay` (`WidgetAnimation.GetEndTime` _pointsanim))
  (`self.K2_DestroyActor`))

(fn `UserConstructionScript`)