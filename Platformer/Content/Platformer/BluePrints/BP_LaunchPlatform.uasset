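; Mushroom launch pad for the platformer that bounces the player into the air when they land on the cap.
; A hit with a straight-down impact normal passes a DoOnce to launch the character, spawn a leap particle and play a timeline that pulses the cap scale.
; A short delay from the timeline update re-arms the DoOnce.
; The construction script scales the cap and stacks stem instances downward to the length of MushBottomEndPoint.
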(event `ResetLauncher`
  (goto _label :!via `Reset`))

(event `self.MushTop.OnComponentHit`
  (params (HitComponent :type "PrimitiveComponent Object Reference") (OtherActor :type "Actor Object Reference") (OtherComp :type "PrimitiveComponent Object Reference") (NormalImpulse :type "Vector Structure") (Hit :type "HitResult Structure (by ref)"))
  (bind _returnvalue (`GameplayStatics.GetPlayerCharacter` 0))
  (bind (_bblockinghit _binitialoverlap _time _distance _location _impactpoint _normal _impactnormal) (`GameplayStatics.BreakHitResult` Hit))
  (if (and (== OtherActor _returnvalue) (`KismetMathLibrary.EqualExactly_VectorVector` _impactnormal (0.0 0.0 -1.0)))
    (`/Engine/EditorBlueprintResources/StandardMacros.DoOnce` false :!label _label
      (:`Completed`
        (`Character.LaunchCharacter` _returnvalue (`self.mushVelocity`) false false)
        (`GameplayStatics.SpawnEmitterAtLocation` "/Game/InfinityBladeEffects/Effects/FX_Skill_Leap/P_Skill_Leap_Base_Launch.P_Skill_Leap_Base_Launch" _impactpoint)
        (bind (_direction _newtrack_0) (`Timeline|PlayerLauncher` :!via `PlayFromStart`)
          (:`Update`
            (`SceneComponent.SetWorldScale3D` (`self.MushTop`) (`KismetMathLibrary.MakeVector` (* (`self.mushScaleX`) _newtrack_0) (* (`self.mushScaleY`) _newtrack_0) (* (`self.mushScaleZ`) _newtrack_0)))
            (`KismetSystemLibrary.Delay` 0.3)
            (`self.ResetLauncher`)))))))

(fn `UserConstructionScript`
  (`SceneComponent.SetWorldScale3D` (`self.MushTop`) (`KismetMathLibrary.MakeVector` (`self.mushScaleX`) (`self.mushScaleY`) (`self.mushScaleZ`)))
  (for _index (range (+ (`KismetMathLibrary.FTrunc` (/ (`KismetMathLibrary.VSize` (`self.MushBottomEndPoint`)) 100.0)) 1))
    (`InstancedStaticMeshComponent.AddInstance` (`self.MushBottom`) (`KismetMathLibrary.MakeTransform` (`KismetMathLibrary.MakeVector` 0.0 0.0 (`KismetMathLibrary.Conv_IntToDouble` (* _index -100)))) false)))