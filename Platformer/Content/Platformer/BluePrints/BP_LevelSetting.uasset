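; BP_LevelSetting runs a platformer level's music, countdown timer and completion flow.
; It binds to game mode respawn, character death and end-flag events, rerunning setup on respawn.
; A looping timer updates the controller's LevelTime, triggers a low-time jingle with faster music, and kills the player at zero.
; Completion pauses the timer, converts remaining time into points tick by tick, then opens the named level.
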(event `player respawn_Event`
  (`AudioComponent.SetPitchMultiplier` (`self.level music component`) 1.0)
  (`self.player respawn`))

(event `player respawn`
  (`|ExecutionSequence` :!label _label
    (:`then_0`
      (bind _asbp_third_person_game_mode (cast `/Game/ThirdPerson/Blueprints/BP_ThirdPersonGameMode` (`GameplayStatics.GetGameMode`)))
      (add `/Game/ThirdPerson/Blueprints/BP_ThirdPersonGameMode.player respawn` _asbp_third_person_game_mode (delegate `player respawn_Event`)))
    (:`then_1`
      (bind _asbp_player_controller (cast `/Game/Platformer/BluePrints/PlayerController/BP_PlayerController` (`GameplayStatics.GetPlayerController` 0)))
      (bind _output_get (set `self.Player Controller ref` _asbp_player_controller))
      (bind _output_get_2 (set `/Game/Platformer/BluePrints/PlayerController/BP_PlayerController.Level time` (`self.time limit max`) _output_get))
      (set `self.time limit current` _output_get_2))
    (:`then_2`
      (`AudioComponent.SetSound` (`self.level music component`) (`self.my level music`))
      (`KismetSystemLibrary.Delay` 0.75)
      (`AudioComponent.Play` (`self.level music component`) 0.0))
    (:`then_3`
      (`KismetSystemLibrary.RetriggerableDelay` 1.0)
      (bind _returnvalue (`KismetSystemLibrary.K2_SetTimerDelegate` (delegate `run level timer`) (`self.time play rate`) true))
      (bind _output_get_3 (set `self.level timer` _returnvalue)))
    (:`then_4`
      (bind _asbp_third_person_character (cast `/Game/ThirdPerson/Blueprints/BP_ThirdPersonCharacter` (`GameplayStatics.GetPlayerCharacter` 0)))
      (add `/Game/ThirdPerson/Blueprints/BP_ThirdPersonCharacter.player start death sequence` _asbp_third_person_character (delegate `player start death sequence_Event`)))
    (:`then_5`
      (add `/Game/Platformer/BluePrints/BP_endOfLevelFlag.level complete` (`self.end of levelflag`) (delegate `level complete_Event`)))))

(event `self.ReceiveBeginPlay`
  (goto _label))

(event `run level timer`
  (bind _level_music_component (`self.level music component`))
  (bind _time_limit_current (`self.time limit current`))
  (if (== _time_limit_current 0)
    (`KismetSystemLibrary.K2_ClearAndInvalidateTimerHandle` (stale `player respawn` _output_get_3))
    (`AudioComponent.Stop` (`self.level music component`))
    (`AudioComponent.Stop` (`self.time runnig out audio`))
    (bind _asbp_third_person_character (cast `/Game/ThirdPerson/Blueprints/BP_ThirdPersonCharacter` (`GameplayStatics.GetPlayerCharacter` 0)))
    (`/Game/ThirdPerson/Blueprints/BP_ThirdPersonCharacter.playerDies` _asbp_third_person_character)
    (else
      (bind _result (`/Engine/EditorBlueprintResources/StandardMacros.DecrementInt` _time_limit_current)
        (:`  `
          (set `/Game/Platformer/BluePrints/PlayerController/BP_PlayerController.Level time` _result (`self.Player Controller ref`))
          (if (== _time_limit_current (`self.time running out warning`))
            (`AudioComponent.SetPaused` (`self.level music component`) true)
            (`AudioComponent.Play` (`self.time runnig out audio`) 0.0)
            (`KismetSystemLibrary.Delay` 2.8)
            (`AudioComponent.SetPaused` _level_music_component false)
            (`AudioComponent.SetPitchMultiplier` _level_music_component 1.05)))))))

(event `player start death sequence_Event`
  (`AudioComponent.Stop` (`self.level music component`))
  (`AudioComponent.Stop` (`self.time runnig out audio`))
  (`KismetSystemLibrary.K2_ClearAndInvalidateTimerHandle` (`self.level timer`)))

(event `level complete_Event`
  (bind _player_controller_ref (`self.Player Controller ref`))
  (`AudioComponent.Stop` (`self.level music component`))
  (`AudioComponent.Stop` (`self.time runnig out audio`))
  (`KismetSystemLibrary.K2_PauseTimerHandle` (`self.level timer`))
  (`KismetSystemLibrary.Delay` 3.0)
  (`ActorComponent.Activate` (`self.level completed`) false)
  (`KismetSystemLibrary.Delay` 0.05 :!label _label_2)
  (bind _result (`/Engine/EditorBlueprintResources/StandardMacros.DecrementInt` (`/Game/Platformer/BluePrints/PlayerController/BP_PlayerController.Level time` _player_controller_ref))
    (:`  `
      (if (> _result 0)
        (`/Game/Platformer/BluePrints/PlayerController/BP_PlayerController.AddPoints` _player_controller_ref 50)
        (`GameplayStatics.PlaySound2D` "/Engine/VREditor/Sounds/UI/Camera_Shutter.Camera_Shutter" 1.0 1.0 0.0 null null)
        (goto _label_2)
        (else
          (`KismetSystemLibrary.Delay` 2.0)
          (`GameplayStatics.OpenLevel` (`self.Level Name`)))))))

(fn `UserConstructionScript`)