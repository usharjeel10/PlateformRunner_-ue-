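; BP_CoinPickup is a coin collectible for a platformer that the player picks up by touching it.
; On BeginPlay it caches the player's BP_PlayerController and enables input, which only drives a debug print on the Q key.
; When the player character overlaps its Sphere, it passes its Coin value to the controller's CoinPickup, spawns an explosion effect, plays a coin sound and destroys itself.
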(event `self.ReceiveBeginPlay`
  (bind _returnvalue (`GameplayStatics.GetPlayerController` 0))
  (bind _asbp_player_controller (cast `/Game/Platformer/BluePrints/PlayerController/BP_PlayerController` _returnvalue))
  (set `self.As BP Player Controller` _asbp_player_controller)
  (`self.EnableInput` _returnvalue))

(event `Key|Q`
  (params (Key :type "Key Structure"))
  (:`Pressed`
    (`KismetSystemLibrary.PrintString` "p key press")))

(event `self.Sphere.OnComponentBeginOverlap`
  (params (OverlappedComponent :type "PrimitiveComponent Object Reference") (OtherActor :type "Actor Object Reference") (OtherComp :type "PrimitiveComponent Object Reference") (OtherBodyIndex :type Integer) (bFromSweep :type Boolean) (SweepResult :type "HitResult Structure (by ref)"))
  (if (== (`GameplayStatics.GetPlayerCharacter` 0) OtherActor)
    (`/Game/Platformer/BluePrints/PlayerController/BP_PlayerController.coinPickup` (`self.As BP Player Controller`) (`self.Coin`))
    (`GameplayStatics.SpawnEmitterAtLocation` "/Game/StarterContent/Particles/P_Explosion.P_Explosion" (`self.K2_GetActorLocation`))
    (`GameplayStatics.PlaySound2D` "/Game/Platformer/audio/Mario_Coin.Mario_Coin" 1.0 1.0 0.0 null null)
    (`self.K2_DestroyActor`)))

(fn `UserConstructionScript`)