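; Mario-style end-of-level flagpole that, on character overlap, disables input, calls level completion and plays a scripted finish sequence.
; It aligns flag or player height, freezes movement, then slides both down the pole with MoveComponentTo.
; The character jumps to an explosion point and is hidden.
; If the level timer's last digit matches FireworksShowSpecial, a self-recalling event loop spawns that many point-awarding fireworks at random box positions.
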(event `self.ReceiveBeginPlay`
  (bind _asbp_player_controller (cast `/Game/Platformer/BluePrints/PlayerController/BP_PlayerController` (`GameplayStatics.GetPlayerController` 0)))
  (set `self.my controller` _asbp_player_controller))

(event `self.trigger volume.OnComponentBeginOverlap`
  (params (OverlappedComponent :type "PrimitiveComponent Object Reference") (OtherActor :type "Actor Object Reference") (OtherComp :type "PrimitiveComponent Object Reference") (OtherBodyIndex :type Integer) (bFromSweep :type Boolean) (SweepResult :type "HitResult Structure (by ref)"))
  (bind _player_end_point (`self.player end point`))
  (bind _flagendpoint (`self.flagEndPoint`))
  (bind _player_explored_point (`self.player explored point`))
  (bind _my_character (`self.my character`))
  (bind _fireworks_area (`self.fireworks area`))
  (bind _firework_locate (`self.firework locate`))
  (bind _fireworks_point (`self.fireworks point`))
  (bind _flag (`self.flag`))
  (bind _my_character_2 (`self.my character`))
  (bind _mesh (`Character.Mesh` (`self.my character`)))
  (bind _capsulecomponent (`Character.CapsuleComponent` (`self.my character`)))
  (bind _capsulecomponent_2 (`Character.CapsuleComponent` _my_character_2))
  (bind _charactermovement (`Character.CharacterMovement` _my_character_2))
  (bind _returnvalue (`SceneComponent.K2_GetComponentLocation` _capsulecomponent))
  (bind _x (.x (`SceneComponent.K2_GetComponentLocation` (`self.flag`))))
  (bind _y (.y (`SceneComponent.K2_GetComponentLocation` (`self.flag`))))
  (bind _z (.z (`SceneComponent.K2_GetComponentLocation` (`self.flag`))))
  (bind _z_2 (.z (`SceneComponent.K2_GetComponentLocation` (`/Game/ThirdPerson/Blueprints/BP_ThirdPersonCharacter.flag attach point` (`self.my character`)))))
  (bind _asbp_third_person_character (cast `/Game/ThirdPerson/Blueprints/BP_ThirdPersonCharacter` OtherActor))
  (bind _output_get (set `self.my character` _asbp_third_person_character))
  (`self.DisableInput` _output_get (`GameplayStatics.GetPlayerController` 0))
  (`/Engine/EditorBlueprintResources/StandardMacros.DoOnce` false
    (:`Completed`
      (`self.level complete`)
      (if (> _z_2 _z)
        (bind _output_get_2 (set `self.flag start point` (`KismetMathLibrary.MakeVector` _x _y _z)))
        (`SceneComponent.K2_SetWorldLocation` _flag _output_get_2 false false)
        (`SceneComponent.K2_SetWorldLocation` (`Character.CapsuleComponent` (`self.my character`)) (`SceneComponent.K2_GetComponentLocation` (`self.player start point`)) false false)
        (else
          (bind _output_get_3 (set `self.flag start point` (`KismetMathLibrary.MakeVector` _x _y _z_2)))
          (`SceneComponent.K2_SetWorldLocation` _flag _output_get_3 false false)))
      (`SceneComponent.K2_SetWorldRotation` _capsulecomponent_2 (`SceneComponent.K2_GetComponentRotation` (`self.player end point`)) false false)
      (`SceneComponent.K2_AddLocalOffset` _capsulecomponent_2 (0.0 30.0 0.0) false false)
      (set `CharacterMovementComponent.GravityScale` 0.0 _charactermovement)
      (`ActorComponent.Deactivate` _charactermovement)
      (`SkeletalMeshComponent.PlayAnimation` _mesh "/Game/Characters/Mannequins/Animations/Manny/MM_Run_Fwd.MM_Run_Fwd" false)
      (`SkeletalMeshComponent.SetPosition` _mesh 1.9 true)
      (`KismetSystemLibrary.Delay` 1.0)
      (`GameplayStatics.PlaySound2D` "/Game/Platformer/audio/Mario_FlagPole.Mario_FlagPole" 1.0 1.0 0.0 null null)
      (`|ExecutionSequence`
        (:`then_0`
          (`KismetSystemLibrary.MoveComponentTo` (`Character.CapsuleComponent` (`self.my character`)) (`SceneComponent.K2_GetComponentLocation` _player_end_point) (`SceneComponent.K2_GetComponentRotation` _player_end_point) false false 1.0)
          (`SkeletalMeshComponent.PlayAnimation` (`Character.Mesh` (`self.my character`)) "/Game/Characters/Mannequins/Animations/Manny/MM_Jump.MM_Jump" false)
          (`KismetSystemLibrary.Delay` 0.3)
          (`SkeletalMeshComponent.PlayAnimation` (`Character.Mesh` _my_character) "/Game/Characters/Mannequins/Animations/Manny/MM_Fall_Loop.MM_Fall_Loop" false)
          (`KismetSystemLibrary.MoveComponentTo` (`Character.CapsuleComponent` _my_character) (`SceneComponent.K2_GetComponentLocation` _player_explored_point) (`SceneComponent.K2_GetComponentRotation` _player_explored_point) false false 0.5)
          (`GameplayStatics.SpawnEmitterAtLocation` "/Game/StarterContent/Particles/P_Explosion.P_Explosion" _returnvalue (struct) (2.0 2.0 2.0))
          (`GameplayStatics.PlaySoundAtLocation` "/Game/StarterContent/Audio/Explosion_Cue.Explosion_Cue" _returnvalue (struct) 1.0 1.0 0.0 null null null null)
          (`SceneComponent.SetVisibility` _capsulecomponent false true)
          (if (== (`self.fireworks show special #`) (`KismetStringLibrary.Right` (`KismetStringLibrary.Conv_IntToString` (`/Game/Platformer/BluePrints/PlayerController/BP_PlayerController.Level time` (`self.my controller`))) 1))
            (`KismetSystemLibrary.Delay` 0.5 :!label _label)
            (`/Engine/EditorBlueprintResources/StandardMacros.Do N` (`self.fireworks show special #`)
              (:`Exit`
                (bind _output_get_4 (set `self.firework locate` (`KismetMathLibrary.RandomPointInBoundingBox` (`SceneComponent.K2_GetComponentLocation` _fireworks_area) (`BoxComponent.BoxExtent` _fireworks_area))))
                (`GameplayStatics.SpawnEmitterAtLocation` "/Game/InfinityBladeEffects/Effects/FX_Monsters/FX_Monster_GolemBot/Notifies/P_SparkBurst.P_SparkBurst" _output_get_4 (struct) (10.0 10.0 10.0))
                (`GameplayStatics.PlaySoundAtLocation` "/Game/Platformer/audio/Mario_Thwomp.Mario_Thwomp" _firework_locate (struct) 1.0 1.0 0.0 null null null null)
                (`|SpawnActorFromClass` "/Game/Platformer/BluePrints/BP_PointsSpawn.BP_PointsSpawn_C" (`KismetMathLibrary.MakeTransform` _firework_locate) "Undefined" "MultiplyWithRoot" null _fireworks_point null)
                (`/Game/Platformer/BluePrints/PlayerController/BP_PlayerController.AddPoints` (`self.my controller`) _fireworks_point)
                (`self.more fireworks`)))))
        (:`then_1`
          (`KismetSystemLibrary.MoveComponentTo` (`self.flag`) (`SceneComponent.RelativeLocation` _flagendpoint) (`SceneComponent.RelativeRotation` _flagendpoint) false false 1.0))))))

(event `more fireworks`
  (goto _label))

(fn `UserConstructionScript`)