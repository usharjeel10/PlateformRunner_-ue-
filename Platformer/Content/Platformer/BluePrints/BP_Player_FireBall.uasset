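; BP_Player_FireBall is the player's bouncing fireball projectile in the platformer.
; On each ProjectileMovement bounce it checks the absolute Z of the impact normal to tell floor-like surfaces from steep ones.
; Steep hits explode it at once, while flat hits raise a bounce counter until its limit triggers the same explosion.
; The explosion spawns a particle effect with attached sound, then destroys the actor.
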(event `self.ProjectileMovement.OnProjectileBounce`
  (params (ImpactResult :type "HitResult Structure (by ref)") (ImpactVelocity :type "Vector Structure (by ref)"))
  (bind (_returnvalue_x _returnvalue_y _returnvalue_z) (`KismetMathLibrary.BreakVector` (`KismetMathLibrary.Vector_GetAbs` (`.Normal` (`GameplayStatics.BreakHitResult` ImpactResult)))))
  (if (< _returnvalue_z 0.8)
    (bind _returnvalue (`GameplayStatics.SpawnEmitterAtLocation` "/Game/StarterContent/Particles/P_Explosion.P_Explosion" (`SceneComponent.K2_GetComponentLocation` (`self.Sphere`)) :!label _label))
    (`GameplayStatics.SpawnSoundAttached` "/Game/StarterContent/Audio/Explosion01.Explosion01" _returnvalue "None" (0.0 0.0 0.0) (struct) "KeepRelativeOffset" false 1.0 1.0 0.0 null null)
    (`self.K2_DestroyActor`)
    (else
      (bind _result (`/Engine/EditorBlueprintResources/StandardMacros.IncrementInt` (`self.fireBallBounceCounter`))
        (:`  `
          (if (not (< _result 2))
            (goto _label)))))))

(fn `UserConstructionScript`)