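; Mario-style warp pipe actor that carries the third-person player to a warp destination.
; An overlap volume opens a gate, letting down or up input (chosen by IsPipeDown) trigger the warp.
; Timelines slide the player's capsule into the pipe, then out rising or falling, with warp sounds and player input disabled until the exit finishes.
; The construction script stacks instanced pipe segments downward, counted from PipeEndPoint's vector length.
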(event `self.ReceiveBeginPlay`
  (`self.EnableInput` (`GameplayStatics.GetPlayerController` 0)))

(event `EnhancedInput|/Game/ThirdPerson/Input/Actions/IA_PlayerDown`
  (params (ActionValue :type Boolean) (ElapsedSeconds :type "Float (double-precision)") (TriggeredSeconds :type "Float (double-precision)") (InputAction :type "InputAction Object Reference" :default "/Game/ThirdPerson/Input/Actions/IA_PlayerDown.IA_PlayerDown"))
  (:`Triggered`
    (if (and (not (`self.is pipe down`)) (`self.can  interact`))
      (`/Engine/EditorBlueprintResources/StandardMacros.Gate` true :!label _label
        (:`Exit`
          (bind _output_get (set `self.My player` (stale `self.collision.OnComponentBeginOverlap` _asbp_third_person_character)))
          (`self.DisableInput` _output_get null)
          (if (`self.is pipe down`)
            (`|ExecutionSequence`
              (:`then_0`
                ;[0 0 0] Enter down pipe
                (bind (_direction _movement) (`Timeline|into the pipe` :!via `PlayFromStart`)
                  (:`Update`
                    (`SceneComponent.K2_SetRelativeLocationAndRotation` :`self` (`Character.CapsuleComponent` (`self.My player`)) :`NewLocation` (`KismetMathLibrary.MakeVector` (.x (`SceneComponent.K2_GetComponentLocation` (`self.wrap IN points`))) (.y (`SceneComponent.K2_GetComponentLocation` (`self.wrap IN points`))) (+ (.z (`SceneComponent.K2_GetComponentLocation` (`self.wrap IN points`))) _movement))))
                  (:`Finished`
                    (`KismetSystemLibrary.Delay` 0.2 :!label _label_2)
                    (`GameplayStatics.PlaySound2D` "/Game/Platformer/audio/Mario_Warp.Mario_Warp" 1.0 1.0 0.0 null null)
                    (if (`self.exit rising up out of pipe`)
                      ;[0 0 0] Exit rising up out of pipe
                      (bind (_direction_2 _movement_2) (`Timeline|Timeline_0` :!via `PlayFromStart`)
                        (:`Update`
                          (`SceneComponent.K2_SetRelativeLocationAndRotation` :`self` (`Character.CapsuleComponent` (`self.My player`)) :`NewLocation` (`KismetMathLibrary.MakeVector` (.x (`self.warpto locale`)) (.y (`self.warpto locale`)) (+ (.z (`self.warpto locale`)) _movement_2))))
                        (:`Finished`
                          (`self.EnableInput` (`GameplayStatics.GetPlayerCharacter` 0) (`GameplayStatics.GetPlayerController` 0) :!label _label_3)))
                      (else
                        ;[0 0 0] exit falling down out of pipe
                        (bind (_direction_3 _movement_3) (`Timeline|Timeline` :!via `PlayFromStart`)
                          (:`Update`
                            (`SceneComponent.K2_SetRelativeLocationAndRotation` :`self` (`Character.CapsuleComponent` (`self.My player`)) :`NewLocation` (`KismetMathLibrary.MakeVector` (.x (`self.warpto locale`)) (.y (`self.warpto locale`)) (+ (.z (`self.warpto locale`)) _movement_3))))
                          (:`Finished`
                            (goto _label_3))))))))
              (:`then_1`
                (`KismetSystemLibrary.Delay` 0.2 :!label _label_4)
                (`GameplayStatics.PlaySound2D` "/Game/Platformer/audio/Mario_Warp.Mario_Warp" 1.0 1.0 0.0 null null)))
            (else
              (`|ExecutionSequence`
                (:`then_0`
                  ;[0 0 0] Enter UP pipe
                  (bind (_direction_4 _movement_4) (`Timeline|Timeline_1` :!via `PlayFromStart`)
                    (:`Update`
                      (`SceneComponent.K2_SetRelativeLocationAndRotation` :`self` (`Character.CapsuleComponent` (`self.My player`)) :`NewLocation` (`KismetMathLibrary.MakeVector` (.x (`self.pipe end point`)) (.y (`self.pipe end point`)) (+ (.z (`self.pipe end point`)) _movement_4))))
                    (:`Finished`
                      (goto _label_2))))
                (:`then_1`
                  (goto _label_4))))))))))

(event `EnhancedInput|/Game/ThirdPerson/Input/Actions/IA_playerUP`
  (params (ActionValue :type Boolean) (ElapsedSeconds :type "Float (double-precision)") (TriggeredSeconds :type "Float (double-precision)") (InputAction :type "InputAction Object Reference" :default "/Game/ThirdPerson/Input/Actions/IA_playerUP.IA_playerUP"))
  (:`Triggered`
    (if (and (`self.is pipe down`) (`self.can  interact`))
      (goto _label))))

(event `self.collision.OnComponentBeginOverlap`
  (params (OverlappedComponent :type "PrimitiveComponent Object Reference") (OtherActor :type "Actor Object Reference") (OtherComp :type "PrimitiveComponent Object Reference") (OtherBodyIndex :type Integer) (bFromSweep :type Boolean) (SweepResult :type "HitResult Structure (by ref)"))
  (bind _asbp_third_person_character (cast `/Game/ThirdPerson/Blueprints/BP_ThirdPersonCharacter` OtherActor))
  (goto _label :!via `Open`))

(event `self.collision.OnComponentEndOverlap`
  (params (OverlappedComponent :type "PrimitiveComponent Object Reference") (OtherActor :type "Actor Object Reference") (OtherComp :type "PrimitiveComponent Object Reference") (OtherBodyIndex :type Integer))
  (cast `/Game/ThirdPerson/Blueprints/BP_ThirdPersonCharacter` OtherActor)
  (goto _label :!via `Close`))

(fn `UserConstructionScript`
  (for _index (range (+ (`KismetMathLibrary.FTrunc` (/ (`KismetMathLibrary.VSize` (`self.pipe end point`)) 100.0)) 1))
    (`InstancedStaticMeshComponent.AddInstance` (`self.pipeBody`) (`KismetMathLibrary.MakeTransform` (`KismetMathLibrary.MakeVector` 0.0 0.0 (`KismetMathLibrary.Conv_IntToDouble` (* _index -100)))) false)))