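; Player controller for a platformer that creates the HUD and tracks coins, points and lives.
; Coin pickups add to the count, and reaching 100 triggers an extra life with a 1-up sound through AdjustLives.
; AdjustLives clamps the life total and opens the main menu level at zero.
; The Enhanced Input pause action toggles the pause menu, cursor and game pause, using cursor visibility as the paused state.
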(event `self.ReceiveBeginPlay`
  (bind _returnvalue (`|CreateWidget` "/Game/Platformer/UI/HUD.HUD_C"))
  (`UserWidget.AddToViewport` _returnvalue 0))

(event `coinPickup`
  (params (coin :type Integer))
  (bind _returnvalue (+ (`self.coin`) coin))
  (if (>= _returnvalue 100)
    (set `self.coin` (`KismetMathLibrary.Clamp` (- (`self.coin`) -100) 0 100))
    (`self.AdjustLives` 1)
    (`GameplayStatics.PlaySound2D` "/Game/Platformer/audio/Mario_1up.Mario_1up" 1.0 1.0 0.0 null null)
    (else
      (set `self.coin` (`KismetMathLibrary.Clamp` _returnvalue 0 1000)))))

(event `AddPoints`
  (params (points :type Integer))
  ;[0 0 0] Add Points
  (set `self.points` (+ (`self.points`) points)))

(event `EnhancedInput|/Game/ThirdPerson/Input/Actions/IA_Pause`
  (params (ActionValue :type Boolean) (ElapsedSeconds :type "Float (double-precision)") (TriggeredSeconds :type "Float (double-precision)") (InputAction :type "InputAction Object Reference" :default "/Game/ThirdPerson/Input/Actions/IA_Pause.IA_Pause"))
  (:`Started`
    (if (`self.bShowMouseCursor`)
      (`Widget.RemoveFromParent` (`self.pausemenu`))
      (set `self.bShowMouseCursor` false)
      (`GameplayStatics.PlaySound2D` "/Game/Platformer/audio/Mario_Pause.Mario_Pause" 1.0 1.0 0.0 null null)
      (`GameplayStatics.SetGamePaused` false)
      (else
        (bind _returnvalue (`|CreateWidget` "/Game/Platformer/UI/pauseMenu.pauseMenu_C"))
        (bind _output_get (set `self.pausemenu` _returnvalue))
        (`UserWidget.AddToViewport` _output_get 0)
        (set `self.bShowMouseCursor` true)
        (`GameplayStatics.PlaySound2D` "/Game/Platformer/audio/Mario_Pause.Mario_Pause" 1.0 1.0 0.0 null null)
        (`GameplayStatics.SetGamePaused` true)))))

(event `AdjustLives`
  (params (`lives to add or subtract` :type Integer))
  ;[0 0 0] Adjust lives script
  (bind _output_get (set `self.lives` (`KismetMathLibrary.Clamp` (+ `lives to add or subtract` (`self.lives`)) 0 100)))
  (if (== _output_get 0)
    (`GameplayStatics.OpenLevel` "LV_MainMenu")))

(fn `UserConstructionScript`)