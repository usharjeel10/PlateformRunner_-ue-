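; One-way platformer platform that the player can jump up through from below and drop down through from on top.
; A top trigger tracks whether the player stands on it, letting the down input disable the platform's collision.
; A bottom trigger disables that collision while the player overlaps it and restores it on exit, which is also the only re-enable path after a drop.
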(event `self.CollisionTop.OnComponentBeginOverlap`
  (params (OverlappedComponent :type "PrimitiveComponent Object Reference") (OtherActor :type "Actor Object Reference") (OtherComp :type "PrimitiveComponent Object Reference") (OtherBodyIndex :type Integer) (bFromSweep :type Boolean) (SweepResult :type "HitResult Structure (by ref)"))
  ;[1 1 1] CheckPlayerOnPlatform
  (if (== OtherActor (`GameplayStatics.GetPlayerCharacter` 0))
    (set `self.Is Player On Platform ?` true)))

(event `self.CollisionTop.OnComponentEndOverlap`
  (params (OverlappedComponent :type "PrimitiveComponent Object Reference") (OtherActor :type "Actor Object Reference") (OtherComp :type "PrimitiveComponent Object Reference") (OtherBodyIndex :type Integer))
  ;[1 1 1] CheckPlayerOnPlatform
  (if (== OtherActor (`GameplayStatics.GetPlayerCharacter` 0))
    (set `self.Is Player On Platform ?` false)))

(event `self.CollisionBottom.OnComponentBeginOverlap`
  (params (OverlappedComponent :type "PrimitiveComponent Object Reference") (OtherActor :type "Actor Object Reference") (OtherComp :type "PrimitiveComponent Object Reference") (OtherBodyIndex :type Integer) (bFromSweep :type Boolean) (SweepResult :type "HitResult Structure (by ref)"))
  ;[1 1 1] JumpOverPlatform
  (if (== OtherActor (`GameplayStatics.GetPlayerCharacter` 0))
    (`PrimitiveComponent.SetCollisionEnabled` (`self.Platform`) "NoCollision")))

(event `self.CollisionBottom.OnComponentEndOverlap`
  (params (OverlappedComponent :type "PrimitiveComponent Object Reference") (OtherActor :type "Actor Object Reference") (OtherComp :type "PrimitiveComponent Object Reference") (OtherBodyIndex :type Integer))
  ;[1 1 1] JumpOverPlatform
  (if (== OtherActor (`GameplayStatics.GetPlayerCharacter` 0))
    (`PrimitiveComponent.SetCollisionEnabled` (`self.Platform`) "QueryAndPhysics")))

(event `EnhancedInput|/Game/ThirdPerson/Input/Actions/IA_PlayerDown`
  (params (ActionValue :type Boolean) (ElapsedSeconds :type "Float (double-precision)") (TriggeredSeconds :type "Float (double-precision)") (InputAction :type "InputAction Object Reference" :default "/Game/ThirdPerson/Input/Actions/IA_PlayerDown.IA_PlayerDown"))
  ;[1 1 1] AllowPlayerDropFromPlatform
  (:`Started`
    (if (`self.Is Player On Platform ?`)
      (`PrimitiveComponent.SetCollisionEnabled` (`self.Platform`) "NoCollision"))))

(fn `UserConstructionScript`)