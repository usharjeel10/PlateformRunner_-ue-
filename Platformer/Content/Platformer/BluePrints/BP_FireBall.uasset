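; BP_FireBall is a rotating chain of fireballs that acts as a platformer hazard, changing the player's hit points on contact.
; The construction script stacks instanced meshes along local Z, stretches the overlap box over them and sets the rotation rate from variables.
; Overlap with player 0 calls AdjustHitPoint on the cached character and sets the rotating movement's Velocity, gated by a DoOnce that resets after a cooldown.
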(event `self.ReceiveBeginPlay`
  (bind _asbp_third_person_character (cast `/Game/ThirdPerson/Blueprints/BP_ThirdPersonCharacter` (`GameplayStatics.GetPlayerCharacter` 0)))
  (set `self.PlayerRef` _asbp_third_person_character))

(event `self.Box.OnComponentBeginOverlap`
  (params (OverlappedComponent :type "PrimitiveComponent Object Reference") (OtherActor :type "Actor Object Reference") (OtherComp :type "PrimitiveComponent Object Reference") (OtherBodyIndex :type Integer) (bFromSweep :type Boolean) (SweepResult :type "HitResult Structure (by ref)"))
  (if (== (`GameplayStatics.GetPlayerCharacter` 0) OtherActor)
    (`/Engine/EditorBlueprintResources/StandardMacros.DoOnce` false :!label _label
      (:`Completed`
        (set `MovementComponent.Velocity` (`self.Velocity`) (`self.RotatingMovement`))
        (`/Game/ThirdPerson/Blueprints/BP_ThirdPersonCharacter.AdjustHitPoint` (`self.PlayerRef`) (`self.HitPoints`))
        (`KismetSystemLibrary.Delay` (`self.coolDown`))
        (goto _label :!via `Reset`)))))

(fn `UserConstructionScript`
  (bind _box (`self.Box`))
  (for _index (range (`self.FlameballNumber`))
    (`|ExecutionSequence`
      (:`then_0`
        (bind _returnvalue (* _index (`self.FlameBallDistAppart`)))
        (`InstancedStaticMeshComponent.AddInstance` (`self.InstancedStaticMesh`) (`KismetMathLibrary.MakeTransform` (`KismetMathLibrary.MakeVector` 0.0 0.0 (`KismetMathLibrary.Conv_IntToDouble` _returnvalue)) (struct) (`self.FlameBallSize`)) false))
      (:`then_1`
        (bind _returnvalue_2 (`KismetMathLibrary.Conv_IntToDouble` (/ _returnvalue 2)))
        (`BoxComponent.SetBoxExtent` _box (`KismetMathLibrary.MakeVector` 10.0 60.0 _returnvalue_2) true)
        (`SceneComponent.K2_SetRelativeLocation` _box (`KismetMathLibrary.MakeVector` 0.0 0.0 _returnvalue_2) false false))
      (:`then_2`
        (set `RotatingMovementComponent.RotationRate` (`self.rotatingRate`) (`self.RotatingMovement`))))))