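; Goomba-style platformer enemy that damages the player on overlap and dies to stomps or fireballs, awarding points with an explosion.
; A top-face Stompbox hit from the player squashes the flipbook before a delayed destroy.
; Tick drives a gate, opened by any detection overlap and closed when the player leaves, that seeks the player or walks sideways.
; Side capsule hits flip direction with a cooldown; construction scales animation rate from Speed.
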(event `self.ReceiveBeginPlay`
  (bind _asbp_player_controller (cast `/Game/Platformer/BluePrints/PlayerController/BP_PlayerController` (`GameplayStatics.GetPlayerController` 0)))
  (set `self.Player Controller` _asbp_player_controller))

(event `self.collider.OnComponentBeginOverlap`
  (params (OverlappedComponent :type "PrimitiveComponent Object Reference") (OtherActor :type "Actor Object Reference") (OtherComp :type "PrimitiveComponent Object Reference") (OtherBodyIndex :type Integer) (bFromSweep :type Boolean) (SweepResult :type "HitResult Structure (by ref)"))
  (bind _asbp_third_person_character (cast `/Game/ThirdPerson/Blueprints/BP_ThirdPersonCharacter` OtherActor))
  (`/Game/ThirdPerson/Blueprints/BP_ThirdPersonCharacter.AdjustHitPoint` _asbp_third_person_character (`self.health_To_Subtract`)))

(event `self.stompbox.OnComponentHit`
  (params (HitComponent :type "PrimitiveComponent Object Reference") (OtherActor :type "Actor Object Reference") (OtherComp :type "PrimitiveComponent Object Reference") (NormalImpulse :type "Vector Structure") (Hit :type "HitResult Structure (by ref)"))
  (bind _points (`self.points`))
  (bind _paperflipbook (`self.PaperFlipbook`))
  (if (and (== OtherActor (`GameplayStatics.GetPlayerCharacter` 0)) (== (`.ImpactNormal` (`GameplayStatics.BreakHitResult` Hit)) (0.0 0.0 -1.0) :`ErrorTolerance` 0.1))
    (`|ExecutionSequence`
      (:`then_0`
        (`GameplayStatics.PlaySound2D` "/Game/Platformer/audio/Mario_Squish.Mario_Squish" 1.0 1.0 0.0 null null)
        (`PrimitiveComponent.SetCollisionEnabled` (`self.collider`) "NoCollision")
        (`ActorComponent.K2_DestroyComponent` (`self.stompbox`))
        (`SceneComponent.SetWorldScale3D` _paperflipbook (0.25 0.25 0.1))
        (`SceneComponent.K2_AddWorldOffset` _paperflipbook (0.0 0.0 -35.0) false false)
        (`CharacterMovementComponent.DisableMovement` (`self.CharacterMovement`)))
      (:`then_1`
        (`|SpawnActorFromClass` "/Game/Platformer/BluePrints/BP_PointsSpawn.BP_PointsSpawn_C" (`self.GetTransform`) "Undefined" "MultiplyWithRoot" null _points null)
        (`/Game/Platformer/BluePrints/PlayerController/BP_PlayerController.AddPoints` (`self.Player Controller`) _points))
      (:`then_2`
        (`KismetSystemLibrary.Delay` 0.5)
        (`/Game/Platformer/BluePrints/BP_LibraryFun.playBlockInteractSound` "/Game/StarterContent/Audio/Explosion_Cue.Explosion_Cue" null "/Game/InfinityBladeEffects/Effects/FX_Monsters/FX_Monster_Gruntling/FlameThrower/P_FlameExplode.P_FlameExplode" (`SceneComponent.K2_GetComponentLocation` (`self.collider`)))
        (`self.K2_DestroyActor`)))))

(event `self.collider.OnComponentHit`
  (params (HitComponent :type "PrimitiveComponent Object Reference") (OtherActor :type "Actor Object Reference") (OtherComp :type "PrimitiveComponent Object Reference") (NormalImpulse :type "Vector Structure") (Hit :type "HitResult Structure (by ref)"))
  (bind _points (`self.points`))
  (bind _asbp_player_fire_ball (cast `/Game/Platformer/BluePrints/BP_Player_FireBall` OtherActor))
  (`self.K2_DestroyActor` _asbp_player_fire_ball)
  (`|ExecutionSequence`
    (:`then_0`
      (`|SpawnActorFromClass` "/Game/Platformer/BluePrints/BP_PointsSpawn.BP_PointsSpawn_C" (`self.GetTransform`) "Undefined" "MultiplyWithRoot" null _points null)
      (`/Game/Platformer/BluePrints/PlayerController/BP_PlayerController.AddPoints` (`self.Player Controller`) _points))
    (:`then_1`
      (`/Game/Platformer/BluePrints/BP_LibraryFun.playBlockInteractSound` "/Game/StarterContent/Audio/Explosion_Cue.Explosion_Cue" null "/Game/InfinityBladeEffects/Effects/FX_Monsters/FX_Monster_Gruntling/FlameThrower/P_FlameExplode.P_FlameExplode" (`SceneComponent.K2_GetComponentLocation` (`self.collider`)))
      (`self.K2_DestroyActor`))))

(event `self.playerDetectRange.OnComponentBeginOverlap`
  (params (OverlappedComponent :type "PrimitiveComponent Object Reference") (OtherActor :type "Actor Object Reference") (OtherComp :type "PrimitiveComponent Object Reference") (OtherBodyIndex :type Integer) (bFromSweep :type Boolean) (SweepResult :type "HitResult Structure (by ref)"))
  (if true
    (goto _label :!via `Open`)))

(event `self.ReceiveTick`
  (params (DeltaSeconds :type "Float (single-precision)"))
  (`/Engine/EditorBlueprintResources/StandardMacros.Gate` true :!label _label
    (:`Exit`
      (if (`self.is seeker`)
        (`AIBlueprintHelperLibrary.SimpleMoveToActor` (`self.GetController`) (`GameplayStatics.GetPlayerCharacter` 0))
        (else
          (`self.AddMovementInput` (select `bool` (`self.move left ?`) :`false` (1.0 0.0 0.0) :`true` (-1.0 0.0 0.0) :!type "Vector Structure"))
          (`PaperFlipbookComponent.SetPlayRate` (`self.PaperFlipbook`) (`self.flipbook play rate multiplier`)))))))

(event `self.playerDetectRange.OnComponentEndOverlap`
  (params (OverlappedComponent :type "PrimitiveComponent Object Reference") (OtherActor :type "Actor Object Reference") (OtherComp :type "PrimitiveComponent Object Reference") (OtherBodyIndex :type Integer))
  (if (== OtherActor (`GameplayStatics.GetPlayerCharacter` 0))
    (goto _label :!via `Close`)))

(event `self.CapsuleComponent.OnComponentHit`
  (params (HitComponent :type "PrimitiveComponent Object Reference") (OtherActor :type "Actor Object Reference") (OtherComp :type "PrimitiveComponent Object Reference") (NormalImpulse :type "Vector Structure") (Hit :type "HitResult Structure (by ref)"))
  (`/Engine/EditorBlueprintResources/StandardMacros.DoOnce` false :!label _label_2
    (:`Completed`
      (if (== (`KismetMathLibrary.Vector_GetAbs` (`.ImpactNormal` (`GameplayStatics.BreakHitResult` Hit))) (1.0 0.0 0.0) :`ErrorTolerance` 0.1)
        (`/Engine/EditorBlueprintResources/StandardMacros.FlipFlop`
          (:`A`
            (set `self.move left ?` false))
          (:`B`
            (set `self.move left ?` true)))
        (`KismetSystemLibrary.Delay` 0.5)
        (goto _label_2 :!via `Reset`)))))

(fn `UserConstructionScript`
  (bind _output_get (set `CharacterMovementComponent.MaxWalkSpeed` (`self.speed`) (`self.CharacterMovement`)))
  (set `self.flipbook play rate multiplier` (`KismetMathLibrary.FClamp` (/ _output_get 100.0) 0.1 3.0)))