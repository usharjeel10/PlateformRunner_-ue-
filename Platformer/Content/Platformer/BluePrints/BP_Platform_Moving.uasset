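; BP_Platform_Moving is a platform actor that moves between two positions in the platformer.
; On BeginPlay it sets the PlatformMovement timeline's play rate from PlayRate and starts it.
; Each timeline update sets the Platform component's relative location by lerping from StartPov to EndPov using the track value, without sweeping.
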(event `self.ReceiveBeginPlay`
  ;[1 1 1] movingPlatform
  (`TimelineComponent.SetPlayRate` (`self.PlatformMovement`) (`self.PlayRate`))
  (bind (_direction _newtrack_0) (`Timeline|PlatformMovement`)
    (:`Update`
      (`SceneComponent.K2_SetRelativeLocation` (`self.Platform`) (`KismetMathLibrary.VLerp` (`self.StartPov`) (`self.EndPov`) _newtrack_0) false false))))

(fn `UserConstructionScript`
  (`parent.UserConstructionScript`))