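; Mario-style fire flower block for the platformer that reveals a power-up when hit.
; The first HitBlock plays interact effects, swaps the material and runs timelines for the block and flower, then adds a glow; later hits only beep.
; Overlapping the flower's box grants the third-person character the flower power-up, spawns and awards points, then destroys the flower and glow components.
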(event `/Game/Platformer/BluePrints/INT_Platform.hitBlock`
  (if (`self.finishedInteracting`)
    (`GameplayStatics.PlaySound2D` "/Game/Platformer/audio/Mario_Beep.Mario_Beep" 1.0 1.0 0.0 null null)
    (else
      (`|ExecutionSequence`
        (:`then_0`
          ;[0.01562 0.01562 0.01562] 0) play sound
          (`/Game/Platformer/BluePrints/BP_LibraryFun.playBlockInteractSound` (`self.interactSFX`) null (`self.interactVFX(particles)`) (+ (`self.K2_GetActorLocation`) (0.0 0.0 50.0)))
          (`PrimitiveComponent.SetMaterial` (`self.blockBase`) 0 (`self.InteractMaterial`)))
        (:`then_1`
          ;[0 0 0] 3) block Anim
          (bind (_direction _movement) (`Timeline|blockAnim`)
            (:`Update`
              (`SceneComponent.K2_SetRelativeLocation` (`self.blockBase`) (`KismetMathLibrary.MakeVector` 0.0 0.0 _movement) false false))
            (:`Finished`
              (bind _returnvalue (`GameplayStatics.SpawnEmitterAtLocation` "/Game/InfinityBladeEffects/Effects/FX_Treasure/Gold_Bag/P_DeadMans_Loot.P_DeadMans_Loot" (`SceneComponent.K2_GetComponentLocation` (`self.meshFlower`))))
              (set `self.powerUpGlow` _returnvalue))))
        (:`then_2`
          ;[0 0 0] 2) flower Anim
          (bind (_direction_2 _movement_2) (`Timeline|flowerAnim`)
            (:`Update`
              (bind _boxflower (`self.BoxFlower`)
                (:`then`
                  (`SceneComponent.K2_SetRelativeLocation` _boxflower (`KismetMathLibrary.MakeVector` 0.0 0.0 _movement_2) false false))
                (:`else`)))))
        (:`then_3`
          (set `self.finishedInteracting` true))))))

(event `self.BoxFlower.OnComponentBeginOverlap`
  (params (OverlappedComponent :type "PrimitiveComponent Object Reference") (OtherActor :type "Actor Object Reference") (OtherComp :type "PrimitiveComponent Object Reference") (OtherBodyIndex :type Integer) (bFromSweep :type Boolean) (SweepResult :type "HitResult Structure (by ref)"))
  (bind _asbp_third_person_character (cast `/Game/ThirdPerson/Blueprints/BP_ThirdPersonCharacter` OtherActor))
  (`/Game/ThirdPerson/Blueprints/BP_ThirdPersonCharacter.got flower powerups` _asbp_third_person_character)
  (`|ExecutionSequence`
    (:`then_0`
      ;[0 0 0] 0) Add points
      (`|SpawnActorFromClass` "/Game/Platformer/BluePrints/BP_PointsSpawn.BP_PointsSpawn_C" (`SceneComponent.K2_GetComponentToWorld` (`self.Arrow`)) "Undefined" "MultiplyWithRoot" null (`self.points`) null)
      (`/Game/Platformer/BluePrints/PlayerController/BP_PlayerController.AddPoints` (`self.Player Controller`) (`self.points`)))
    (:`then_1`
      ;[0 0 0] destroy components
      (bind _boxflower (`self.BoxFlower`)
        (:`then`
          (bind _powerupglow (`self.powerUpGlow`)
            (:`then`
              (bind _meshflower (`self.meshFlower`)
                (:`then`
                  (`ActorComponent.K2_DestroyComponent` _meshflower)
                  (`ActorComponent.K2_DestroyComponent` _powerupglow)
                  (`ActorComponent.K2_DestroyComponent` _boxflower))
                (:`else`)))
            (:`else`)))
        (:`else`)))))

(fn `UserConstructionScript`
  (`parent.UserConstructionScript`))