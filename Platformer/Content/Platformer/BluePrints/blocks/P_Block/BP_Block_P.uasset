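; P-switch style platformer block that the player stomps from above to temporarily switch on tagged BP_BlockBase actors.
; A stomp bounces the character, plays effects, swaps in the smashed meshes and replaces level music with its own track.
; A timer, the player's death sequence or level completion switches the blocks off and resumes level music, via bound events sharing one cleanup path.
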(event `self.Box.OnComponentHit`
  (params (HitComponent :type "PrimitiveComponent Object Reference") (OtherActor :type "Actor Object Reference") (OtherComp :type "PrimitiveComponent Object Reference") (NormalImpulse :type "Vector Structure") (Hit :type "HitResult Structure (by ref)"))
  (bind _asbp_third_person_character (cast `/Game/ThirdPerson/Blueprints/BP_ThirdPersonCharacter` OtherActor))
  (if (== (`.ImpactNormal` (`GameplayStatics.BreakHitResult` Hit)) (0.0 0.0 -1.0) :`ErrorTolerance` 0.01)
    (`Character.LaunchCharacter` _asbp_third_person_character (0.0 0.0 400.0) false false)
    (`|ExecutionSequence`
      (:`then_0`
        (`GameplayStatics.PlaySound2D` null 1.0 1.0 0.0 null null)
        (`GameplayStatics.SpawnEmitterAtLocation` "/Game/InfinityBladeEffects/Effects/FX_Breakables/pot/P_PotBreak_Ceramic.P_PotBreak_Ceramic" (`SceneComponent.K2_GetComponentLocation` (`self.Block_P_Base_Samashed`)))
        (`AudioComponent.Play` (`self.music`) 0.0)
        (`AudioComponent.SetPaused` (`/Game/Platformer/BluePrints/BP_LevelSetting.level music component` (`self.level setting`)) true))
      (:`then_1`
        (`GameplayStatics.PlayWorldCameraShake` null (`self.K2_GetActorLocation` (`GameplayStatics.GetPlayerCharacter` 0)) 1000.0 2000.0)
        (`PlayerController.K2_ClientPlayForceFeedback` (`GameplayStatics.GetPlayerController` 0) "/Game/Platformer/BluePrints/blocks/P_Block/NewForceFeedbackEffect.NewForceFeedbackEffect" "None" false false false))
      (:`then_2`
        (`SceneComponent.SetVisibility` (`self.Block_P_Base_Samashed`) true false)
        (`SceneComponent.SetVisibility` (`self.Block_P_UP_Samashed`) true false)
        (`ActorComponent.K2_DestroyComponent` (`self.Box`))
        (`ActorComponent.K2_DestroyComponent` (`self.block_P`)))
      (:`then_3`
        (bind _outactors (`GameplayStatics.GetAllActorsWithTag` (`self.tag`)))
        (bind _output_get (set `self.p_blocks` _outactors))
        (for _array_element _output_get
          (bind _asbp_block_base (cast `/Game/Platformer/BluePrints/blocks/BP_BlockBase` _array_element))
          (`/Game/Platformer/BluePrints/blocks/BP_BlockBase.FBlockON` _asbp_block_base)))
      (:`then_4`
        (`KismetSystemLibrary.K2_SetTimerDelegate` (delegate `p block timer over`) (`self.P_Block time duration`)))
      (:`then_5`
        (add `/Game/ThirdPerson/Blueprints/BP_ThirdPersonCharacter.player start death sequence` _asbp_third_person_character (delegate `player start death sequence_Event`)))
      (:`then_6`
        (add `/Game/Platformer/BluePrints/BP_endOfLevelFlag.level complete` (`self.end of level flag`) (delegate `level complete_Event`))))))

(event `p block timer over`
  (for _array_element (`self.p_blocks`) :!label _label
    (bind _asbp_block_base (cast `/Game/Platformer/BluePrints/blocks/BP_BlockBase` _array_element))
    (`/Engine/EditorBlueprintResources/StandardMacros.IsValid` _asbp_block_base
      (:`Is Valid`
        (`/Game/Platformer/BluePrints/blocks/BP_BlockBase.FblockOFF` _asbp_block_base))
      (:`Is Not Valid`
        _))
    (`AudioComponent.Stop` (`self.music`))
    (`AudioComponent.SetPaused` (`/Game/Platformer/BluePrints/BP_LevelSetting.level music component` (`self.level setting`)) false)))

(event `player start death sequence_Event`
  (goto _label))

(event `level complete_Event`
  (goto _label))

(fn `UserConstructionScript`)