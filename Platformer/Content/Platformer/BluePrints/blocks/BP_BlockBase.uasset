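; BP_BlockBase is a base platformer block that reacts to player contact.
; It calls HitBlockMessage when the player character hits it with an impact normal Z of exactly 1, and destroys itself when the player overlaps CoinCollider.
; FBlockON and FblockOFF, not called here, swap visibility between the block and its ChildActor and toggle block collision.
; BeginPlay caches the BP_PlayerController reference.
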(event `self.ReceiveBeginPlay`
  ;[1 1 1] ref To player Controller
  (bind _asbp_player_controller (cast `/Game/Platformer/BluePrints/PlayerController/BP_PlayerController` (`GameplayStatics.GetPlayerController` 0)))
  (set `self.Player Controller` _asbp_player_controller))

(event `self.blockBase.OnComponentHit`
  (params (HitComponent :type "PrimitiveComponent Object Reference") (OtherActor :type "Actor Object Reference") (OtherComp :type "PrimitiveComponent Object Reference") (NormalImpulse :type "Vector Structure") (Hit :type "HitResult Structure (by ref)"))
  (if (and (== OtherActor (`GameplayStatics.GetPlayerCharacter` 0)) (== (.z (`.ImpactNormal` (`GameplayStatics.BreakHitResult` Hit))) 1.0))
    (message `/Game/Platformer/BluePrints/INT_Platform.hitBlock` self)))

(event `self.coin collider.OnComponentBeginOverlap`
  (params (OverlappedComponent :type "PrimitiveComponent Object Reference") (OtherActor :type "Actor Object Reference") (OtherComp :type "PrimitiveComponent Object Reference") (OtherBodyIndex :type Integer) (bFromSweep :type Boolean) (SweepResult :type "HitResult Structure (by ref)"))
  (if (== OtherActor (`GameplayStatics.GetPlayerCharacter` 0))
    (`self.K2_DestroyActor`)))

(fn `FblockOFF`
  (`SceneComponent.SetVisibility` (`self.blockBase`) true false)
  (`PrimitiveComponent.SetCollisionEnabled` (`self.blockBase`) "QueryAndPhysics")
  (`SceneComponent.SetVisibility` (`self.ChildActor`) false false))

(fn `FBlockON`
  (bind _blockbase (`self.blockBase`))
  (`SceneComponent.SetVisibility` _blockbase false false)
  (`PrimitiveComponent.SetCollisionEnabled` _blockbase "NoCollision")
  (`SceneComponent.SetVisibility` (`self.ChildActor`) true false))

(fn `UserConstructionScript`)