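; Breakable platformer block that, when hit, either shatters or bumps depending on the player character's HitPoints.
; At two or more HitPoints, HitBlock plays the interact sound and particles, spawns a BP_PointsSpawn, adds the points through the player controller and destroys the block.
; Otherwise it plays a beep and a timeline moves the block mesh along its relative Z axis.
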(event `/Game/Platformer/BluePrints/INT_Platform.hitBlock`
  (bind _asbp_third_person_character (cast `/Game/ThirdPerson/Blueprints/BP_ThirdPersonCharacter` (`GameplayStatics.GetPlayerCharacter` 0)))
  (if (>= (`/Game/ThirdPerson/Blueprints/BP_ThirdPersonCharacter.HitPoints` _asbp_third_person_character) 2)
    (`|ExecutionSequence`
      (:`then_0`
        (`/Game/Platformer/BluePrints/BP_LibraryFun.playBlockInteractSound` (`self.interactSFX`) null (`self.interactVFX(particles)`) (`self.K2_GetActorLocation`)))
      (:`then_1`
        (`|SpawnActorFromClass` "/Game/Platformer/BluePrints/BP_PointsSpawn.BP_PointsSpawn_C" (`self.GetTransform`) "Undefined" "MultiplyWithRoot" null (`self.points`) null)
        (`/Game/Platformer/BluePrints/PlayerController/BP_PlayerController.AddPoints` (`self.Player Controller`) (`self.points`)))
      (:`then_2`
        (`self.K2_DestroyActor`)))
    (else
      (`GameplayStatics.PlaySound2D` "/Game/Platformer/audio/Mario_Beep.Mario_Beep" 1.0 1.0 0.0 null null)
      (bind (_direction _movement) (`Timeline|Timeline` :!via `PlayFromStart`)
        (:`Update`
          (`SceneComponent.K2_SetRelativeLocation` (`self.blockBase`) (`KismetMathLibrary.MakeVector` 0.0 0.0 _movement) false false))))))

(fn `UserConstructionScript`
  (`parent.UserConstructionScript`))