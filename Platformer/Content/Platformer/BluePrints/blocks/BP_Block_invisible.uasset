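; Hidden Mario-style coin block that starts invisible, ignoring one trace channel, and reveals itself when hit.
; Each hit spawns points and coin actors, credits the player controller and plays a timeline bump.
; The first hit starts a timer; the first hit after it expires gives a last reward, swaps the material and leaves later hits only beeping.
; Player overlap with Box disables block collision; the re-enable and interact SFX/VFX nodes are unwired.
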(event `self.ReceiveBeginPlay`
  (bind _blockbase (`self.blockBase`))
  (`parent.ReceiveBeginPlay`)
  (`SceneComponent.SetVisibility` _blockbase false false)
  (`PrimitiveComponent.SetCollisionResponseToChannel` _blockbase "ECC_GameTraceChannel1" "ECR_Ignore"))

(event `CustomEvent`
  (set `self.IsInteractFinished` true))

(event `/Game/Platformer/BluePrints/INT_Platform.hitBlock`
  (bind _blockbase (`self.blockBase`))
  (if (`self.finishedInteracting`)
    (`GameplayStatics.PlaySound2D` "/Game/Platformer/audio/Mario_Beep.Mario_Beep" 1.0 1.0 0.0 null null)
    (elif (`self.IsInteractFinished`)
      (`/Engine/EditorBlueprintResources/StandardMacros.DoOnce` false
        (:`Completed`
          (`|ExecutionSequence`
            (:`then_0`
              (`|ExecutionSequence` :!label _label
                (:`then_0`
                  (`/Engine/EditorBlueprintResources/StandardMacros.DoOnce` false
                    (:`Completed`
                      (`KismetSystemLibrary.K2_SetTimerDelegate` (delegate `CustomEvent`) (`self.interactTime`)))))
                (:`then_1`
                  ;[0 0 0] 1) Add points
                  (`|SpawnActorFromClass` "/Game/Platformer/BluePrints/BP_PointsSpawn.BP_PointsSpawn_C" (`self.GetTransform`) "Undefined" "MultiplyWithRoot" null (`self.points`) null)
                  (`/Game/Platformer/BluePrints/PlayerController/BP_PlayerController.AddPoints` (`self.Player Controller`) (`self.points`)))
                (:`then_2`
                  ;[0 0 0] 2)add coins
                  (`|SpawnActorFromClass` "/Game/Platformer/BluePrints/blocks/BP_BlockCoin.BP_BlockCoin_C" (`self.GetTransform`) "Undefined" "MultiplyWithRoot" null null)
                  (`/Game/Platformer/BluePrints/PlayerController/BP_PlayerController.coinPickup` (`self.Player Controller`) (`self.coinsToAdd`)))
                (:`then_3`
                  ;[0 0 0] 3) block Anim
                  (bind (_direction _movement) (`Timeline|blockAnim`)
                    (:`Update`
                      (`SceneComponent.K2_SetRelativeLocation` (`self.blockBase`) (`KismetMathLibrary.MakeVector` 0.0 0.0 _movement) false false))))
                (:`then_4`
                  ;[0 0 0] 4) visibile box
                  (`SceneComponent.SetVisibility` _blockbase true false)
                  (`PrimitiveComponent.SetCollisionResponseToChannel` _blockbase "ECC_GameTraceChannel1" "ECR_Block"))))
            (:`then_1`
              (`PrimitiveComponent.SetMaterial` (`self.blockBase`) 0 (`self.InteractMaterial`))
              (set `self.finishedInteracting` true)))))
      (else
        (goto _label)))))

(event `self.Box.OnComponentBeginOverlap`
  (params (OverlappedComponent :type "PrimitiveComponent Object Reference") (OtherActor :type "Actor Object Reference") (OtherComp :type "PrimitiveComponent Object Reference") (OtherBodyIndex :type Integer) (bFromSweep :type Boolean) (SweepResult :type "HitResult Structure (by ref)"))
  (bind _blockbase (`self.blockBase`))
  (if (== OtherActor (`GameplayStatics.GetPlayerCharacter` 0))
    (`/Engine/EditorBlueprintResources/StandardMacros.IsValid` _blockbase
      (:`Is Valid`
        (`PrimitiveComponent.SetCollisionEnabled` _blockbase "NoCollision")))))

(event `self.Box.OnComponentEndOverlap`
  (params (OverlappedComponent :type "PrimitiveComponent Object Reference") (OtherActor :type "Actor Object Reference") (OtherComp :type "PrimitiveComponent Object Reference") (OtherBodyIndex :type Integer))
  (if (== (`GameplayStatics.GetPlayerCharacter` 0) OtherActor)
    (`/Engine/EditorBlueprintResources/StandardMacros.IsValid` (`self.blockBase`))))

(fn `UserConstructionScript`
  (`parent.UserConstructionScript`))