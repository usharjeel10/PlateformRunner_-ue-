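; BP_Block_Fake_BreakAble is a platformer block that pays out points and coins on its first hit instead of breaking.
; HitBlock plays interact sound and particles, swaps the material, spawns point and coin actors, and credits both through the PlayerController.
; A BlockAnim timeline bumps the mesh along Z.
; A FinishedInteracting flag then limits later hits to a beep sound.
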(event `/Game/Platformer/BluePrints/INT_Platform.hitBlock`
  (if (`self.finishedInteracting`)
    (`GameplayStatics.PlaySound2D` "/Game/Platformer/audio/Mario_Beep.Mario_Beep" 1.0 1.0 0.0 null null)
    (else
      (`|ExecutionSequence`
        (:`then_0`
          ;[0.01562 0.01562 0.01562] 0) play sound
          (`/Game/Platformer/BluePrints/BP_LibraryFun.playBlockInteractSound` (`self.interactSFX`) null (`self.interactVFX(particles)`) (+ (`self.K2_GetActorLocation`) (0.0 0.0 50.0)))
          (`PrimitiveComponent.SetMaterial` (`self.blockBase`) 0 (`self.InteractMaterial`)))
        (:`then_1`
          ;[0 0 0] 1) Add points
          (`|SpawnActorFromClass` "/Game/Platformer/BluePrints/BP_PointsSpawn.BP_PointsSpawn_C" (`self.GetTransform`) "Undefined" "MultiplyWithRoot" null (`self.points`) null)
          (`/Game/Platformer/BluePrints/PlayerController/BP_PlayerController.AddPoints` (`self.Player Controller`) (`self.points`)))
        (:`then_2`
          ;[0 0 0] 2)add coins
          (`|SpawnActorFromClass` "/Game/Platformer/BluePrints/blocks/BP_BlockCoin.BP_BlockCoin_C" (`self.GetTransform`) "Undefined" "MultiplyWithRoot" null null)
          (`/Game/Platformer/BluePrints/PlayerController/BP_PlayerController.coinPickup` (`self.Player Controller`) (`self.coinsToAdd`)))
        (:`then_3`
          ;[1 1 1] 3) block Anim
          (bind (_direction _movement) (`Timeline|blockAnim`)
            (:`Update`
              (`SceneComponent.K2_SetRelativeLocation` (`self.blockBase`) (`KismetMathLibrary.MakeVector` 0.0 0.0 _movement) false false))))
        (:`then_4`
          (set `self.finishedInteracting` true))))))

(fn `UserConstructionScript`
  (`parent.UserConstructionScript`))