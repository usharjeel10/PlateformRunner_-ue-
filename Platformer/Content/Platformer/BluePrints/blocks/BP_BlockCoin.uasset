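; BP_BlockCoin is a short-lived coin effect actor for the platformer's blocks.
; On BeginPlay it plays the CoinAnim timeline, which drives the Coin component's relative height and yaw from Movement and Rotation tracks.
; When the timeline finishes, it spawns the P_Loot_Pickup particle emitter at the coin's location and destroys itself.
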(event `self.ReceiveBeginPlay`
  (`TimelineComponent.SetPlayRate` (`self.coinAnim`) 1.0)
  (bind (_direction _movement _rotation) (`Timeline|coinAnim` :!via `PlayFromStart`)
    (:`Update`
      (`SceneComponent.K2_SetRelativeLocationAndRotation` (`self.coin`) (`KismetMathLibrary.MakeVector` 0.0 0.0 _movement) (`KismetMathLibrary.MakeRotator` 0.0 0.0 _rotation) false false))
    (:`Finished`
      (`GameplayStatics.SpawnEmitterAtLocation` "/Game/InfinityBladeEffects/Effects/FX_Treasure/Loot/P_Loot_Pickup.P_Loot_Pickup" (`SceneComponent.K2_GetComponentLocation` (`self.coin`)))
      (`self.K2_DestroyActor`))))

(fn `UserConstructionScript`)